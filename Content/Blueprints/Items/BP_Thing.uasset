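; BP_Thing is an item actor that continuously spins and drifts, with all motion driven in Tick from an accumulated ElapsedTime.
; Yaw is set from elapsed time times RotationRate, with pitch and roll held at zero.
; Each frame it adds an unswept world offset of Perlin noise on Y and a SineRate and SineAmp sine wave on Z.
; These offsets are not scaled by DeltaSeconds, so movement depends on frame rate.
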(event EventBeginPlay)

(event Collision|EventActorBeginOverlap
  (params (OtherActor :type Actor%20Object%20Reference)))

(event EventTick
  (params (DeltaSeconds :type Float%20%28single-precision%29))
  (bind _output_get (Variables|Default|SetElapsed%20Time (+ DeltaSeconds (Variables|Default|GetElapsed%20Time))))
  (Transformation|SetActorRotation (Math|Rotator|MakeRotator 0.0 0.0 (* _output_get (Variables|Default|GetRotation%20Rate))))
  (Transformation|AddActorWorldOffset (Math|Vector|MakeVector 0.0 (* (Class|KismetMathLibrary|PerlinNoise1D (* _output_get 1.0)) 1.0) (* (Math|Trig|Sin(Degrees) (* _output_get (Variables|Default|GetSine%20Rate))) (Variables|Default|GetSine%20Amp)))))

(fn ConstructionScript)